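; NBCharacterBase is a character Blueprint that follows the player.
; On BeginPlay it runs the parent logic, then caches the player as TargetPlayer.
; Each Tick it snaps its full rotation to look at that target with a teleporting rotation set.
; While more than 300 units away, it adds forward movement input, moving directly toward the player without pathfinding.
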(event `self.ReceiveBeginPlay`
  (`parent.ReceiveBeginPlay`)
  (bind _asmaster (`/Game/HorrorEngine/Blueprints/Core/HorrorEngineFunctions.GetPlayer`))
  (set `self.TargetPlayer` _asmaster))

(event `self.ReceiveTick`
  (params (DeltaSeconds :type "Float (single-precision)"))
  (bind _returnvalue (`self.K2_GetActorLocation`))
  (bind _returnvalue_2 (`self.K2_GetActorLocation` (`self.TargetPlayer`)))
  (`self.K2_SetActorRotation` (`KismetMathLibrary.FindLookAtRotation` _returnvalue _returnvalue_2) true)
  (if (> (`KismetMathLibrary.Vector_Distance` _returnvalue _returnvalue_2) 300.0)
    (`self.AddMovementInput` (`KismetMathLibrary.GetForwardVector` (`self.K2_GetActorRotation`)))))

(fn `UserConstructionScript`)